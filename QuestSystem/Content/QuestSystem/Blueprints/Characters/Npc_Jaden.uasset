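; Npc_Jaden is a quest system NPC whose dialogue changes after the player first talks to him.
; OnTalkto always passes the interaction to the parent class.
; On the first talk it also sets a TalkenTo flag and, after the parent call, overwrites the default message and duration, so later talks use a reminder to go and help others.
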(event EventBeginPlay
  (|CallParentFunction))

(event Collision|EventActorBeginOverlap
  (params (OtherActor :type Actor%20Object%20Reference)))

(event EventTick
  (params (DeltaSeconds :type Float%20%28single-precision%29)))

(event EventOnTalkto
  (params (Player :type Third%20Person%20Character%20Object%20Reference))
  (if (Variables|Default|GetTalkenTo?)
    (|CallParentFunction Player)
    (else
      (Variables|Default|SetTalkenTo? true)
      (|CallParentFunction Player)
      (Variables|Default|SetDefaultMessage "Please, go and try to help them.")
      (Variables|Default|SetDefaultDuration 3.0))))

(fn ConstructionScript
  (|CallParentFunction))