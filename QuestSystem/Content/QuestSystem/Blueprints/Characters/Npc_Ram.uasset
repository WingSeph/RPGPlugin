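; Ram NPC Blueprint for the quest system that overrides its parent's talk behavior with quest-aware dialogue.
; When talked to, it asks the player's quest manager whether Quest_Test1 is a current quest with goal index 2 among its current goals.
; If so, it shows a short congratulatory message; otherwise it falls back to the parent's talk handling.
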(event EventBeginPlay
  (|CallParentFunction))

(event Collision|EventActorBeginOverlap
  (params (OtherActor :type Actor%20Object%20Reference)))

(event EventTick
  (params (DeltaSeconds :type Float%20%28single-precision%29)))

(event EventOnTalkto
  (params (Player :type Third%20Person%20Character%20Object%20Reference))
  (bind _questmanagerref (Variables|/Game/QuestSystem/Blueprints/Characters/ThirdPersonCharacter.ThirdPersonCharacter_C|GetQuestManagerRef Player))
  (bind (_out_ _questactor) (Default|HasCurrentQuest? _questmanagerref "/Game/QuestSystem/Blueprints/Actors/QuestActors/Quest_Test1.Quest_Test1_C"))
  (if _out_
    (if (Utilities|Array|ContainsItem (Variables|/Game/QuestSystem/Blueprints/Actors/QuestActors/Bp_MasterQuest.Bp_MasterQuest_C|GetCurrentGoalIndices _questactor) 2)
      (CallFunction|ShowMessage "Ah, now we can talk. Good job!" 3.5 Player)
      (else
        (|CallParentFunction Player :!label _label)))
    (else
      (goto _label))))

(fn ConstructionScript
  (|CallParentFunction))