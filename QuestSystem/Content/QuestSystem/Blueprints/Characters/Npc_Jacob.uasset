(event EventBeginPlay
  (|CallParentFunction))

(event Collision|EventActorBeginOverlap
  (params (OtherActor :type Actor%20Object%20Reference)))

(event EventTick
  (params (DeltaSeconds :type Float%20%28single-precision%29)))

(event EventShowMessage
  (params (Message :type Text) (Duration :type Float%20%28single-precision%29) (Player :type Third%20Person%20Character%20Object%20Reference))
  (if (Variables|Default|GetcanBeTalkedTo?)
    (Variables|Default|SetcanBeTalkedTo? false)
    (Rendering|SetVisibility (Variables|Default|GetInteractionWidget) false false)
    (Rendering|Components|TextRender|SetText (Variables|/Game/QuestSystem/Widgets/MessageWidget.MessageWidget_C|GetMessage (Variables|Default|GetMessageWidget)) Message)
    (Rendering|SetVisibility (Variables|Default|GetMessageComponent) true false)
    (if (Utilities|Array|ContainsItem (Variables|/Game/QuestSystem/Blueprints/Characters/ThirdPersonCharacter.ThirdPersonCharacter_C|GetObtainedObjects (stale EventOnTalkto Player)) "/Game/QuestSystem/Blueprints/Actors/Objects/Object_Chest.Object_Chest_C")
      (Default|OnTalkedtoNpc (Variables|/Game/QuestSystem/Blueprints/Characters/ThirdPersonCharacter.ThirdPersonCharacter_C|GetQuestManagerRef Player) (Utilities|GetClass self) (Variables|Default|GetNpcID)))
    (Utilities|FlowControl|Delay Duration)
    (Rendering|SetVisibility (Variables|Default|GetMessageComponent) false false)
    (Rendering|SetVisibility (Variables|Default|GetInteractionWidget) (Variables|Default|GetinPlayerRadius?) false)
    (Variables|Default|SetcanBeTalkedTo? true)))

(event EventOnTalkto
  (params (Player :type Third%20Person%20Character%20Object%20Reference))
  (if (Utilities|Array|ContainsItem (Variables|/Game/QuestSystem/Blueprints/Characters/ThirdPersonCharacter.ThirdPersonCharacter_C|GetObtainedObjects Player) "/Game/QuestSystem/Blueprints/Actors/Objects/Object_Chest.Object_Chest_C")
    (if (Variables|Default|GetChestReceived?)
      (Variables|Default|SetDefaultMessage "I think there are some other people that also need your help...")
      (|CallParentFunction Player)
      (else
        (Variables|Default|SetChestReceived? true)
        (Variables|Default|SetDefaultMessage "Thank you! Now i can finally get back to work again!")
        (|CallParentFunction Player)))
    (else
      (|CallParentFunction Player))))

(fn ConstructionScript
  (|CallParentFunction))