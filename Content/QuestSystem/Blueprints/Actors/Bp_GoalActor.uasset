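; Quest goal marker actor that shows on the minimap as either a point icon or a colored radius circle.
; The construction script toggles between the two through UseRadius, then scales and tints the circle sprite from Radius and CircleColor.
; On BeginPlay it makes the player character its owner and sets Owner No See on both components, hiding them from that player's own view.
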(event Collision|EventActorBeginOverlap
  (params (OtherActor :type Actor%20Object%20Reference)))

(event EventBeginPlay
  (Actor|SetOwner (Game|GetPlayerCharacter 0))
  (Class|PrimitiveComponent|SetOwnerNoSee (Variables|Default|GetMiniMapIcon) true))

(event EventTick
  (params (DeltaSeconds :type Float%20%28single-precision%29)))

(fn ConstructionScript
  (bind _minimapradius (Variables|Default|GetMiniMapRadius))
  (bind _radius (Variables|Default|GetRadius))
  (bind _returnvalue (/ _radius 5e+02))
  (Rendering|SetVisibility (Variables|Default|GetMiniMapIcon) (not (Variables|Default|GetUseRadius?)) false)
  (Transformation|SetRelativeScale3D _minimapradius (Math|Vector|MakeVector _returnvalue 1.0 _returnvalue))
  (Rendering|SetVisibility _minimapradius (Variables|Default|GetUseRadius?) false)
  (Sprite|SetSpriteColor _minimapradius (Variables|Default|GetCircleColor)))