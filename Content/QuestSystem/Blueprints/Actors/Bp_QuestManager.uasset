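; Quest manager actor that spawns, tracks, selects, cancels and restores quest actors, syncing them with the HUD list and journal.
; Talk, find and kill events advance matching goals, deferring quest-completing ones until the scan of current quests finishes.
; The selected subgoal spawns a goal marker that drives distance text and a map direction arrow.
; Ended quests are re-filed by state, completed ones granting experience and regional prestige.
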(event Custom|OnSwitchSubQuest
  (bind _currentquest (Variables|Default|GetCurrentQuest))
  (bind _mainwidget (Variables|Default|GetMainWidget))
  (Utilities|IsValid (Variables|Default|GetCurrentGoalActor)
    (:Is%20Valid
      (Actor|DestroyActor (Variables|Default|GetCurrentGoalActor)))
    (:Is%20Not%20Valid
      _))
  (bind _output_get (Variables|Default|SetCurrentSubGoal (Utilities|Array|Get(acopy) (.SubGoals (Utilities|Struct|Breaks_QuestInfo (Variables|/Game/QuestSystem/Blueprints/Actors/QuestActors/Bp_MasterQuest.Bp_MasterQuest_C|GetQuestInfo _currentquest))) (Variables|/Game/QuestSystem/Blueprints/Actors/QuestActors/Bp_MasterQuest.Bp_MasterQuest_C|GetSelectedSubGoalIndex _currentquest))))
  (if (.hasLocation? (Utilities|Struct|Breaks_LocationInfo (.Location (Utilities|Struct|BreakGoalInfo _output_get))))
    (bind _returnvalue (Game|SpawnActorfromClass "/Game/QuestSystem/Blueprints/Actors/Bp_GoalActor.Bp_GoalActor_C" (Math|Transform|MakeTransform (.Location (Utilities|Struct|Breaks_LocationInfo (.Location (Utilities|Struct|BreakGoalInfo _output_get)))) "0, 0, 0" "1,1,1") "AlwaysSpawn" 0 (.UseRadius? (Utilities|Struct|BreakGoalInfo _output_get)) (.Radius (Utilities|Struct|BreakGoalInfo _output_get)) (.CircleColor (Utilities|Struct|BreakGoalInfo _output_get))))
    (Variables|Default|SetCurrentGoalActor _returnvalue)
    (bind _output_get_2 (Variables|Default|SetCurrentDistance (CallFunction|DistancetoGoal)))
    (Rendering|Components|TextRender|SetText (Variables|/Game/QuestSystem/Widgets/MainWidget.MainWidget_C|GetDistanceText (Variables|Default|GetMainWidget)) (Utilities|Text|ToText(Integer) _output_get_2 false))
    (CallFunction|UpdateDirectionArrow)
    (Widget|SetVisibility (Variables|/Game/QuestSystem/Widgets/MainWidget.MainWidget_C|GetDistanceBorder _mainwidget) "HitTestInvisible")
    (Widget|SetVisibility (Variables|/Game/QuestSystem/Widgets/MiniMap.MiniMap_C|GetDirectionArrow (Variables|/Game/QuestSystem/Widgets/MainWidget.MainWidget_C|GetMap _mainwidget)) (select (> (Variables|Default|GetCurrentDistance) (Variables|Default|GetShowDirectionArrowAmount)) "HitTestInvisible" "Hidden"))
    (else
      (Variables|Default|SetCurrentGoalActor 0)
      (Widget|SetVisibility (Variables|/Game/QuestSystem/Widgets/MainWidget.MainWidget_C|GetDistanceBorder (Variables|Default|GetMainWidget)) "Hidden"))))

(event Custom|OnTalkedToNpc
  (params (NpcClass :type Master%20Npc%20Class%20Reference) (NpcID :type Integer))
  (Utilities|Array|Clear (Variables|Default|GetIndicesToCompleteLater))
  (for _array_element (Variables|Default|GetCurrentQuestActors)
    (for (_array_element_2 _array_index) (Variables|/Game/QuestSystem/Blueprints/Actors/QuestActors/Bp_MasterQuest.Bp_MasterQuest_C|GetCurrentGoals _array_element)
      (if (Math|Boolean|ANDBoolean (Utilities|Enum|Equal(Enum) (.Type (Utilities|Struct|BreakGoalInfo _array_element_2)) "NewEnumerator3") (== (.GoalClass (Utilities|Struct|BreakGoalInfo _array_element_2)) NpcClass) (== (.GoalId (Utilities|Struct|BreakGoalInfo _array_element_2)) NpcID))
        (if (.CompletesQuest? (Utilities|Struct|BreakGoalInfo _array_element_2))
          (Utilities|Array|Add (Variables|Default|GetIndicesToCompleteLater) (Utilities|Struct|Makes_IndexToComplete _array_element (Utilities|Array|Get(acopy) (Variables|/Game/QuestSystem/Blueprints/Actors/QuestActors/Bp_MasterQuest.Bp_MasterQuest_C|GetCurrentGoalIndices _array_element) _array_index)))
          (else
            (Default|CompleteSubGoal _array_element (Utilities|Array|Get(acopy) (Variables|/Game/QuestSystem/Blueprints/Actors/QuestActors/Bp_MasterQuest.Bp_MasterQuest_C|GetCurrentGoalIndices _array_element) _array_index) false))))))
  (CallFunction|CompleteGoals))

(event Custom|OnEnemyKilled
  (params (Class :type Master%20Enemy%20Class%20Reference))
  (Utilities|Array|Clear (Variables|Default|GetIndicesToCompleteLater))
  (Variables|Default|SetKilledEnemy Class)
  (for _array_element (Variables|Default|GetCurrentQuestActors)
    (for (_array_element_2 _array_index) (Variables|/Game/QuestSystem/Blueprints/Actors/QuestActors/Bp_MasterQuest.Bp_MasterQuest_C|GetCurrentGoals _array_element)
      (if (and (Utilities|Enum|Equal(Enum) (.Type (Utilities|Struct|BreakGoalInfo _array_element_2)) "NewEnumerator1") (== (.GoalClass (Utilities|Struct|BreakGoalInfo _array_element_2)) (Variables|Default|GetKilledEnemy)))
        (if (>= (+ (Utilities|Array|Get(acopy) (Variables|/Game/QuestSystem/Blueprints/Actors/QuestActors/Bp_MasterQuest.Bp_MasterQuest_C|GetCurrentHuntedAmounts _array_element) _array_index) 1) (.AmountToHunt (Utilities|Struct|BreakGoalInfo _array_element_2)))
          (if (.CompletesQuest? (Utilities|Struct|BreakGoalInfo _array_element_2))
            (Utilities|Array|Add (Variables|Default|GetIndicesToCompleteLater) (Utilities|Struct|Makes_IndexToComplete _array_element (Utilities|Array|Get(acopy) (Variables|/Game/QuestSystem/Blueprints/Actors/QuestActors/Bp_MasterQuest.Bp_MasterQuest_C|GetCurrentGoalIndices _array_element) _array_index)))
            (else
              (Default|CompleteSubGoal _array_element (Utilities|Array|Get(acopy) (Variables|/Game/QuestSystem/Blueprints/Actors/QuestActors/Bp_MasterQuest.Bp_MasterQuest_C|GetCurrentGoalIndices _array_element) _array_index) false)))
          (else
            (Utilities|Array|SetArrayElem (Variables|/Game/QuestSystem/Blueprints/Actors/QuestActors/Bp_MasterQuest.Bp_MasterQuest_C|GetCurrentHuntedAmounts _array_element) _array_index (+ (Utilities|Array|Get(acopy) (Variables|/Game/QuestSystem/Blueprints/Actors/QuestActors/Bp_MasterQuest.Bp_MasterQuest_C|GetCurrentHuntedAmounts _array_element) _array_index) 1))
            (Default|Update (Utilities|Array|Get(acopy) (Variables|/Game/QuestSystem/Widgets/QuestWidget.QuestWidget_C|GetSubGoalWidgets (Variables|/Game/QuestSystem/Blueprints/Actors/QuestActors/Bp_MasterQuest.Bp_MasterQuest_C|GetQuestWidget _array_element)) _array_index))
            (if (Default|SelectedinJournal? _array_element)
              (Default|GenerateSubGoals (Variables|/Game/QuestSystem/Widgets/MainWidget.MainWidget_C|GetJournal (Variables|Default|GetMainWidget)))))))))
  (CallFunction|CompleteGoals))

(event Custom|OnPlayerMove
  (Utilities|IsValid (Variables|Default|GetCurrentGoalActor)
    (:Is%20Valid
      (bind _output_get (Variables|Default|SetCurrentDistance (CallFunction|DistancetoGoal)))
      (Rendering|Components|TextRender|SetText (Variables|/Game/QuestSystem/Widgets/MainWidget.MainWidget_C|GetDistanceText (Variables|Default|GetMainWidget)) (Utilities|Text|ToText(Integer) _output_get false))
      (Math|Integer|CompareInt (Variables|Default|GetCurrentDistance) (Variables|Default|GetShowDirectionArrowAmount)
        (:>
          _)
        (:==
          _)
        (:<
          (Utilities|FlowControl|DoOnce false :!label _label
            (:Completed
              (Widget|SetVisibility (Variables|/Game/QuestSystem/Widgets/MiniMap.MiniMap_C|GetDirectionArrow (Variables|/Game/QuestSystem/Widgets/MainWidget.MainWidget_C|GetMap (Variables|Default|GetMainWidget))) "Hidden")
              (goto _label_2 Reset)))))
      (CallFunction|UpdateDirectionArrow)
      (Utilities|FlowControl|DoOnce false :!label _label_2
        (:Completed
          (Widget|SetVisibility (Variables|/Game/QuestSystem/Widgets/MiniMap.MiniMap_C|GetDirectionArrow (Variables|/Game/QuestSystem/Widgets/MainWidget.MainWidget_C|GetMap (Variables|Default|GetMainWidget))) "HitTestInvisible")
          (goto _label Reset))))))

(event Custom|LoadQuests
  (bind _self self)
  (bind _mainwidget (Variables|Default|GetMainWidget))
  (for _array_element (Variables|/Game/QuestSystem/Blueprints/Characters/ThirdPersonCharacter.ThirdPersonCharacter_C|GetLoadedQuests (Variables|Default|GetThirdPersonChar))
    (Utilities|Array|Add (Variables|Default|GetAllQuestClasses) (.QuestClass (Utilities|Struct|Breaks_SavedQuest _array_element)))
    (bind _returnvalue (Game|SpawnActorfromClass (.QuestClass (Utilities|Struct|Breaks_SavedQuest _array_element)) (Math|Transform|MakeTransform "0, 0, 0" "0, 0, 0" "1,1,1") "AlwaysSpawn" 0 self 0))
    (Variables|Default|SetLoadedQuest _returnvalue)
    (Variables|/Game/QuestSystem/Blueprints/Actors/QuestActors/Bp_MasterQuest.Bp_MasterQuest_C|SetCurrentGoalIndices (Variables|Default|GetLoadedQuest) (.CurrentGoalIndices (Utilities|Struct|Breaks_SavedQuest _array_element)))
    (Variables|/Game/QuestSystem/Blueprints/Actors/QuestActors/Bp_MasterQuest.Bp_MasterQuest_C|SetCurrentHuntedAmounts (Variables|Default|GetLoadedQuest) (.HuntAmounts (Utilities|Struct|Breaks_SavedQuest _array_element)))
    (Variables|/Game/QuestSystem/Blueprints/Actors/QuestActors/Bp_MasterQuest.Bp_MasterQuest_C|SetSelectedSubGoalIndex (Variables|Default|GetLoadedQuest) (.SelectedGoalIndex (Utilities|Struct|Breaks_SavedQuest _array_element)))
    (Variables|/Game/QuestSystem/Blueprints/Actors/QuestActors/Bp_MasterQuest.Bp_MasterQuest_C|SetCurrentGoals (Variables|Default|GetLoadedQuest) (.CurrentGoals (Utilities|Struct|Breaks_SavedQuest _array_element)))
    (Variables|/Game/QuestSystem/Blueprints/Actors/QuestActors/Bp_MasterQuest.Bp_MasterQuest_C|SetCurrentDescription (Variables|Default|GetLoadedQuest) (.CurrentDescription (Utilities|Struct|Breaks_SavedQuest _array_element)))
    (Variables|/Game/QuestSystem/Blueprints/Actors/QuestActors/Bp_MasterQuest.Bp_MasterQuest_C|SetCompletedSubGoals (Variables|Default|GetLoadedQuest) (.CompletedGoals (Utilities|Struct|Breaks_SavedQuest _array_element)))
    (Variables|/Game/QuestSystem/Blueprints/Actors/QuestActors/Bp_MasterQuest.Bp_MasterQuest_C|SetCurrentState (Variables|Default|GetLoadedQuest) (.CurrentState (Utilities|Struct|Breaks_SavedQuest _array_element)))
    (Utilities|Array|Add (Utilities|Select :Index (Variables|/Game/QuestSystem/Blueprints/Actors/QuestActors/Bp_MasterQuest.Bp_MasterQuest_C|GetCurrentState (Variables|Default|GetLoadedQuest)) :NewEnumerator0 (Variables|Default|GetCurrentQuestActors) :NewEnumerator1 (Variables|Default|GetCompletedQuestActors) :NewEnumerator2 (Variables|Default|GetFailedQuestActors)) (Variables|Default|GetLoadedQuest))
    (Default|AddEntry (Variables|/Game/QuestSystem/Widgets/MainWidget.MainWidget_C|GetJournal (Variables|Default|GetMainWidget)) (Variables|Default|GetLoadedQuest))
    (if (Utilities|Enum|Equal(Enum) (Variables|/Game/QuestSystem/Blueprints/Actors/QuestActors/Bp_MasterQuest.Bp_MasterQuest_C|GetCurrentState (Variables|Default|GetLoadedQuest)) "NewEnumerator0")
      (bind _widget (Default|AddQuesttoList (Variables|Default|GetMainWidget) (Variables|Default|GetLoadedQuest)))
      (Variables|/Game/QuestSystem/Blueprints/Actors/QuestActors/Bp_MasterQuest.Bp_MasterQuest_C|SetQuestWidget (Variables|Default|GetLoadedQuest) _widget)
      (Default|UpdateQuest _widget)
      (if (.CurrentlyActive? (Utilities|Struct|Breaks_SavedQuest _array_element))
        (CallFunction|SelectNewQuest (Variables|Default|GetLoadedQuest) (Utilities|Array|Get(acopy) (Variables|/Game/QuestSystem/Widgets/QuestWidget.QuestWidget_C|GetSubGoalWidgets _widget) (Utilities|Array|FindItem (Variables|/Game/QuestSystem/Blueprints/Actors/QuestActors/Bp_MasterQuest.Bp_MasterQuest_C|GetCurrentGoalIndices (Variables|Default|GetLoadedQuest)) (Variables|/Game/QuestSystem/Blueprints/Actors/QuestActors/Bp_MasterQuest.Bp_MasterQuest_C|GetSelectedSubGoalIndex (Variables|Default|GetLoadedQuest)))) true)
        (if (Variables|/Game/QuestSystem/Widgets/MainWidget.MainWidget_C|GetSlideOut? _mainwidget)
          (UserInterface|Animation|PlayAnimation _mainwidget (Variables|/Game/QuestSystem/Widgets/MainWidget.MainWidget_C|GetSlideOut _mainwidget) 0.0 1 "Reverse" 1.0)
          (Variables|/Game/QuestSystem/Widgets/MainWidget.MainWidget_C|SetSlideOut? _mainwidget false)))))
  (for _array_element_2 (Variables|Default|GetAllNpcsInWorld)
    (Default|OnQuestsLoaded _array_element_2 _self))
  (for _array_element_3 (Variables|Default|GetAllObjectsInWorld)
    (Default|OnGameLoaded _array_element_3 _self)))

(event Custom|OnObjectFound
  (params (FoundObject :type Master%20Object%20Class%20Reference))
  (Utilities|Array|Clear (Variables|Default|GetIndicesToCompleteLater))
  (Variables|Default|SetFoundObject FoundObject)
  (for _array_element (Variables|Default|GetCurrentQuestActors)
    (for (_array_element_2 _array_index) (Variables|/Game/QuestSystem/Blueprints/Actors/QuestActors/Bp_MasterQuest.Bp_MasterQuest_C|GetCurrentGoals _array_element)
      (if (and (Utilities|Enum|Equal(Enum) (.Type (Utilities|Struct|BreakGoalInfo _array_element_2)) "NewEnumerator2") (== (.GoalClass (Utilities|Struct|BreakGoalInfo _array_element_2)) (Variables|Default|GetFoundObject)))
        (if (.CompletesQuest? (Utilities|Struct|BreakGoalInfo _array_element_2))
          (Utilities|Array|Add (Variables|Default|GetIndicesToCompleteLater) (Utilities|Struct|Makes_IndexToComplete _array_element (Utilities|Array|Get(acopy) (Variables|/Game/QuestSystem/Blueprints/Actors/QuestActors/Bp_MasterQuest.Bp_MasterQuest_C|GetCurrentGoalIndices _array_element) _array_index)))
          (else
            (Default|CompleteSubGoal _array_element (Utilities|Array|Get(acopy) (Variables|/Game/QuestSystem/Blueprints/Actors/QuestActors/Bp_MasterQuest.Bp_MasterQuest_C|GetCurrentGoalIndices _array_element) _array_index) false))))))
  (CallFunction|CompleteGoals))

(event Collision|EventActorBeginOverlap
  (params (OtherActor :type Actor%20Object%20Reference)))

(event EventTick
  (params (DeltaSeconds :type Float%20%28single-precision%29)))

(event EventBeginPlay
  (CallFunction|GetAllNpcs)
  (CallFunction|GetAllObjects))

(fn ConstructionScript)

(fn SelectNewQuest
  (params (Quest :type Bp%20Master%20Quest%20Object%20Reference) (SubGoal :type Sub%20Goal%20Widget%20Object%20Reference) (Loaded? :type Boolean))
  (Utilities|IsValid (Variables|Default|GetCurrentQuest)
    (:Is%20Valid
      (Widget|SetIsEnabled (Variables|/Game/QuestSystem/Widgets/QuestWidget.QuestWidget_C|GetQuestName (Variables|/Game/QuestSystem/Blueprints/Actors/QuestActors/Bp_MasterQuest.Bp_MasterQuest_C|GetQuestWidget (Variables|Default|GetCurrentQuest))) false)
      (Default|SelectSubGoal (Variables|/Game/QuestSystem/Blueprints/Actors/QuestActors/Bp_MasterQuest.Bp_MasterQuest_C|GetQuestWidget (Variables|Default|GetCurrentQuest)) 0 false))
    (:Is%20Not%20Valid
      _))
  (bind _output_get (Variables|Default|SetCurrentQuest Quest))
  (Default|OnQuestSelected (Variables|/Game/QuestSystem/Blueprints/Actors/QuestActors/Bp_MasterQuest.Bp_MasterQuest_C|GetQuestWidget _output_get) SubGoal Loaded?)
  (return))

(fn AddNewQuest
  (params (QuestClass :type Bp%20Master%20Quest%20Class%20Reference) (DirectlyStart? :type Boolean))
  (bind _mainwidget (Variables|Default|GetMainWidget))
  (LocalVariables|SetlocalClass QuestClass)
  (LocalVariables|SetlocalStart? DirectlyStart?)
  (if (and (Utilities|IsValidClass QuestClass) (not (Utilities|Array|ContainsItem (Variables|Default|GetAllQuestClasses) QuestClass)))
    (Utilities|Array|Add (Variables|Default|GetAllQuestClasses) (LocalVariables|GetlocalClass))
    (bind _returnvalue (Game|SpawnActorfromClass (LocalVariables|GetlocalClass) (Math|Transform|MakeTransform "0, 0, 0" "0, 0, 0" "1,1,1") "AlwaysSpawn" 0 self 0))
    (bind _output_get (LocalVariables|SetlocalQuestActor _returnvalue))
    (Utilities|Array|Add (Variables|Default|GetCurrentQuestActors) _output_get)
    (bind _widget (Default|AddQuesttoList (Variables|Default|GetMainWidget) (LocalVariables|GetlocalQuestActor)))
    (bind _output_get_2 (Variables|/Game/QuestSystem/Blueprints/Actors/QuestActors/Bp_MasterQuest.Bp_MasterQuest_C|SetQuestWidget (LocalVariables|GetlocalQuestActor) _widget))
    (Default|SetupStartingGoals (LocalVariables|GetlocalQuestActor))
    (Default|UpdateQuest _output_get_2)
    (Default|AddEntry (Variables|/Game/QuestSystem/Widgets/MainWidget.MainWidget_C|GetJournal (Variables|Default|GetMainWidget)) (LocalVariables|GetlocalQuestActor))
    (if (or (LocalVariables|GetlocalStart?) (<= (Utilities|Array|Length (Variables|Default|GetCurrentQuestActors)) 1))
      (CallFunction|SelectNewQuest (LocalVariables|GetlocalQuestActor) (Utilities|Array|Get(acopy) (Variables|/Game/QuestSystem/Widgets/QuestWidget.QuestWidget_C|GetSubGoalWidgets (Variables|/Game/QuestSystem/Blueprints/Actors/QuestActors/Bp_MasterQuest.Bp_MasterQuest_C|GetQuestWidget (LocalVariables|GetlocalQuestActor)))) false))
    (if (Variables|/Game/QuestSystem/Widgets/MainWidget.MainWidget_C|GetSlideOut? (Variables|Default|GetMainWidget))
      (UserInterface|Animation|PlayAnimation _mainwidget (Variables|/Game/QuestSystem/Widgets/MainWidget.MainWidget_C|GetSlideOut _mainwidget) 0.0 1 "Reverse" 1.0)
      (Variables|/Game/QuestSystem/Widgets/MainWidget.MainWidget_C|SetSlideOut? _mainwidget false)
      (return true)
      (else
        (return true)))
    (else
      (return false))))

(fn DistancetoGoal
  (bind _currentgoalactor (Variables|Default|GetCurrentGoalActor))
  (bind _thirdpersonchar (Variables|Default|GetThirdPersonChar))
  (bind _returnvalue (Transformation|GetActorLocation _thirdpersonchar))
  (bind _returnvalue_2 (Transformation|GetActorLocation _currentgoalactor))
  (return (Math|Float|Round (/ (Math|Vector|VectorLength (- (Math|Vector|MakeVector (.x _returnvalue) (.y _returnvalue) 0.0) (Math|Vector|MakeVector (.x _returnvalue_2) (.y _returnvalue_2) 0.0))) 1e+02))))

(fn UpdateDirectionArrow
  (Class|Widget|SetRenderAngle (Variables|/Game/QuestSystem/Widgets/MiniMap.MiniMap_C|GetDirectionArrow (Variables|/Game/QuestSystem/Widgets/MainWidget.MainWidget_C|GetMap (Variables|Default|GetMainWidget))) (.Yaw (Math|Rotator|BreakRotator (Math|Rotator|FindLookatRotation (Transformation|GetActorLocation (Variables|Default|GetThirdPersonChar)) (Transformation|GetActorLocation (Variables|Default|GetCurrentGoalActor))))))
  (return))

(fn HasCurrentQuest?
  (params (QuestClass :type Bp%20Master%20Quest%20Class%20Reference))
  (bind _array_element (Utilities|Array|ForEachLoopwithBreak (Variables|Default|GetCurrentQuestActors) :!label _label)
    (:LoopBody
      (if (== (Utilities|GetClass _array_element) QuestClass)
        (LocalVariables|SetFoundQuest _array_element)
        (goto _label Break)))
    (:Completed
      (Utilities|IsValid (LocalVariables|GetFoundQuest)
        (:Is%20Valid
          (return true (LocalVariables|GetFoundQuest)))
        (:Is%20Not%20Valid
          (return false 0))))))

(fn EndQuest
  (params (Quest :type Bp%20Master%20Quest%20Object%20Reference))
  (bind _currentgoalactor (Variables|Default|GetCurrentGoalActor))
  (bind _currentquestactors (Variables|Default|GetCurrentQuestActors))
  (bind _thirdpersonchar (Variables|Default|GetThirdPersonChar))
  (bind _item (Utilities|Array|Get(acopy) _currentquestactors))
  (bind _output_get (LocalVariables|SetlocalQuest Quest))
  (Utilities|Array|RemoveItem (Variables|Default|GetCurrentQuestActors) _output_get)
  (Utilities|Array|Add (Utilities|Select :Index (Variables|/Game/QuestSystem/Blueprints/Actors/QuestActors/Bp_MasterQuest.Bp_MasterQuest_C|GetCurrentState (LocalVariables|GetlocalQuest)) :NewEnumerator0 (Variables|Default|GetCurrentQuestActors) :NewEnumerator1 (Variables|Default|GetCompletedQuestActors) :NewEnumerator2 (Variables|Default|GetFailedQuestActors)) (LocalVariables|GetlocalQuest))
  (Default|AddEntry (Variables|/Game/QuestSystem/Widgets/MainWidget.MainWidget_C|GetJournal (Variables|Default|GetMainWidget)) (LocalVariables|GetlocalQuest))
  (if (== (LocalVariables|GetlocalQuest) (Variables|Default|GetCurrentQuest))
    (Variables|Default|SetCurrentQuest 0)
    (Utilities|IsValid _currentgoalactor
      (:Is%20Valid
        (Actor|DestroyActor _currentgoalactor)
        (Widget|SetVisibility (Variables|/Game/QuestSystem/Widgets/MainWidget.MainWidget_C|GetDistanceBorder (Variables|Default|GetMainWidget)) "Hidden"))
      (:Is%20Not%20Valid
        _))
    (Utilities|IsValid _item
      (:Is%20Valid
        (CallFunction|SelectNewQuest _item (Utilities|Array|Get(acopy) (Variables|/Game/QuestSystem/Widgets/QuestWidget.QuestWidget_C|GetSubGoalWidgets (Variables|/Game/QuestSystem/Blueprints/Actors/QuestActors/Bp_MasterQuest.Bp_MasterQuest_C|GetQuestWidget _item))) false))
      (:Is%20Not%20Valid
        _)))
  (if (Default|SelectedinJournal? (LocalVariables|GetlocalQuest))
    (Default|OnQuestClicked (Variables|/Game/QuestSystem/Widgets/MainWidget.MainWidget_C|GetJournal (Variables|Default|GetMainWidget))))
  (if (Utilities|Enum|Equal(Enum) (Variables|/Game/QuestSystem/Blueprints/Actors/QuestActors/Bp_MasterQuest.Bp_MasterQuest_C|GetCurrentState (LocalVariables|GetlocalQuest)) "NewEnumerator1")
    (Default|AddExperiencePoints _thirdpersonchar (.Experience (Utilities|Struct|Breaks_QuestReward (.CompletionReward (Utilities|Struct|Breaks_QuestInfo (Variables|/Game/QuestSystem/Blueprints/Actors/QuestActors/Bp_MasterQuest.Bp_MasterQuest_C|GetQuestInfo (LocalVariables|GetlocalQuest)))))))
    (Default|SetPrestigebyRegion _thirdpersonchar (.Region (Utilities|Struct|Breaks_QuestInfo (Variables|/Game/QuestSystem/Blueprints/Actors/QuestActors/Bp_MasterQuest.Bp_MasterQuest_C|GetQuestInfo (LocalVariables|GetlocalQuest)))) (+ (Default|GetPrestigebyRegion _thirdpersonchar (.Region (Utilities|Struct|Breaks_QuestInfo (Variables|/Game/QuestSystem/Blueprints/Actors/QuestActors/Bp_MasterQuest.Bp_MasterQuest_C|GetQuestInfo (LocalVariables|GetlocalQuest))))) (.PrestigePoints (Utilities|Struct|Breaks_QuestReward (.CompletionReward (Utilities|Struct|Breaks_QuestInfo (Variables|/Game/QuestSystem/Blueprints/Actors/QuestActors/Bp_MasterQuest.Bp_MasterQuest_C|GetQuestInfo (LocalVariables|GetlocalQuest))))))))
    (return)
    (else
      (return))))

(fn CompleteGoals
  (for _array_element (Variables|Default|GetIndicesToCompleteLater)
    (Default|CompleteSubGoal (.Quest (Utilities|Struct|Breaks_IndexToComplete _array_element)) (.Index (Utilities|Struct|Breaks_IndexToComplete _array_element)) false)))

(fn GetAllNpcs
  (bind _outactors (Actor|GetAllActorsOfClass "/Game/QuestSystem/Blueprints/Characters/Master_Npc.Master_Npc_C"))
  (Variables|Default|SetAllNpcsInWorld _outactors)
  (return))

(fn FindNpcbyId
  (params (Class :type Master%20Npc%20Class%20Reference) (Id :type Integer))
  (bind _array_element (Utilities|Array|ForEachLoopwithBreak (Variables|Default|GetAllNpcsInWorld) :!label _label)
    (:LoopBody
      (if (and (== (Utilities|GetClass _array_element) Class) (== (Variables|/Game/QuestSystem/Blueprints/Characters/Master_Npc.Master_Npc_C|GetNpcID _array_element) Id))
        (LocalVariables|SetlocalFoundNpc _array_element)
        (goto _label Break)))
    (:Completed
      (Utilities|IsValid (LocalVariables|GetlocalFoundNpc)
        (:Is%20Valid
          (return true (LocalVariables|GetlocalFoundNpc)))
        (:Is%20Not%20Valid
          (return false 0))))))

(fn CancelQuest
  (params (QuestActor :type Bp%20Master%20Quest%20Object%20Reference))
  (bind _currentgoalactor (Variables|Default|GetCurrentGoalActor))
  (bind _currentquestactors (Variables|Default|GetCurrentQuestActors))
  (bind _item (Utilities|Array|Get(acopy) _currentquestactors))
  (bind _output_get (LocalVariables|SetlocalQuest QuestActor))
  (Utilities|Array|RemoveItem (Variables|Default|GetCurrentQuestActors) _output_get)
  (if (== (LocalVariables|GetlocalQuest) (Variables|Default|GetCurrentQuest))
    (Variables|Default|SetCurrentQuest 0)
    (Utilities|IsValid _currentgoalactor
      (:Is%20Valid
        (Actor|DestroyActor _currentgoalactor)
        (Widget|SetVisibility (Variables|/Game/QuestSystem/Widgets/MainWidget.MainWidget_C|GetDistanceBorder (Variables|Default|GetMainWidget)) "Hidden"))
      (:Is%20Not%20Valid
        _))
    (Utilities|IsValid _item
      (:Is%20Valid
        (CallFunction|SelectNewQuest _item (Utilities|Array|Get(acopy) (Variables|/Game/QuestSystem/Widgets/QuestWidget.QuestWidget_C|GetSubGoalWidgets (Variables|/Game/QuestSystem/Blueprints/Actors/QuestActors/Bp_MasterQuest.Bp_MasterQuest_C|GetQuestWidget _item))) false))
      (:Is%20Not%20Valid
        _)))
  (if (Default|SelectedinJournal? (LocalVariables|GetlocalQuest))
    (Default|OnQuestClicked (Variables|/Game/QuestSystem/Widgets/MainWidget.MainWidget_C|GetJournal (Variables|Default|GetMainWidget))))
  (if (.HasClient? (Utilities|Struct|Breaks_QuestInfo (Variables|/Game/QuestSystem/Blueprints/Actors/QuestActors/Bp_MasterQuest.Bp_MasterQuest_C|GetQuestInfo (LocalVariables|GetlocalQuest))))
    (bind (_found_ _npc) (CallFunction|FindNpcbyId (.ClientClass (Utilities|Struct|Breaks_QuestInfo (Variables|/Game/QuestSystem/Blueprints/Actors/QuestActors/Bp_MasterQuest.Bp_MasterQuest_C|GetQuestInfo (LocalVariables|GetlocalQuest)))) (.ClientId (Utilities|Struct|Breaks_QuestInfo (Variables|/Game/QuestSystem/Blueprints/Actors/QuestActors/Bp_MasterQuest.Bp_MasterQuest_C|GetQuestInfo (LocalVariables|GetlocalQuest))))))
    (if _found_
      (Default|OnOwnQuestCancelled _npc (Utilities|GetClass (LocalVariables|GetlocalQuest)))))
  (Utilities|Array|RemoveItem (Variables|Default|GetAllQuestClasses) (Utilities|GetClass (LocalVariables|GetlocalQuest)))
  (Actor|DestroyActor (LocalVariables|GetlocalQuest))
  (return))

(fn GetAllObjects
  (bind _outactors (Actor|GetAllActorsOfClass "/Game/QuestSystem/Blueprints/Actors/Objects/Master_Object.Master_Object_C"))
  (Variables|Default|SetAllObjectsInWorld _outactors)
  (return))